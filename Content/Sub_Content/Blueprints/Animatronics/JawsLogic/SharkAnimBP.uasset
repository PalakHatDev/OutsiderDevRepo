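; Actor Blueprint for a shark animatronic (Jaws) that animates its jaw, tail and fin, despite the AnimBP name.
; JawFaceMorphs plays a timeline that drives a jaw morph target on MainAnimBody, looked up by key code and scaled by blend amount; BeginPlay also starts it.
; Tick uses random 1–2 second Delays to retrigger timelines that lerp tail yaw and fin height toward random, multiplier-scaled targets for idle motion.
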(event Custom|FinChange
  (params (FinMap :type Float%20%28double-precision%29))
  (bind _mountpointfin (Variables|Default|GetMountPointFin))
  (bind _relativelocation (Variables|/Script/Engine.SceneComponent|GetRelativeLocation _mountpointfin))
  (bind (_x _y _z) (Math|Vector|BreakVector _relativelocation))
  (bind _animtrack (Timeline|Timeline_1 PlayFromStart)
    (:Update
      (Transformation|SetRelativeLocation _mountpointfin (Math|Vector|MakeVector _x _y (Math|Float|Lerp _z (Math|Float|MapRangeClamped (Math|Float|Clamp(Float) (* FinMap (Variables|Default|GetFinAnimMult))) 0.0 1.0 139.740319 179.740319) _animtrack)) false false))))

(event Custom|TailChange
  (params (TailMap :type Float%20%28double-precision%29))
  (bind _tailmountpoint (Variables|Default|GetTailMountPoint))
  (bind _animtrack (Timeline|Timeline_0 PlayFromStart)
    (:Update
      (Transformation|SetRelativeRotation _tailmountpoint (Math|Rotator|MakeRotator 0.0 0.0 (Math|Float|Lerp (.Yaw (Math|Rotator|BreakRotator (Variables|/Script/Engine.SceneComponent|GetRelativeRotation _tailmountpoint))) (Math|Float|MapRangeClamped (Math|Float|Clamp(Float) (* (Variables|Default|GetTailAnimMult) TailMap)) 0.0 1.0 -4e+01 4e+01) _animtrack)) false false))))

(event Custom|JawFaceMorphs
  (params (KeyCode :type Name%20%28by%20ref%29) (BlendAmount :type Float%20%28double-precision%29))
  (bind _animtrack (Timeline|Timeline PlayFromStart)
    (:Update
      (Components|SkeletalMesh|SetMorphTarget (Variables|Default|GetMainAnimBody) (.Value (Utilities|Map|Find (Variables|Default|GetMorphMapsJaw) KeyCode)) (* _animtrack BlendAmount) false))))

(event EventBeginPlay
  (bind _animtrack (Timeline|Timeline PlayFromStart)
    (:Update
      (Components|SkeletalMesh|SetMorphTarget (Variables|Default|GetMainAnimBody) (.Value (Utilities|Map|Find (Variables|Default|GetMorphMapsJaw) (stale Custom|JawFaceMorphs KeyCode))) (* _animtrack (stale Custom|JawFaceMorphs BlendAmount)) false))))

(event Collision|EventActorBeginOverlap
  (params (OtherActor :type Actor%20Object%20Reference)))

(event EventTick
  (params (DeltaSeconds :type Float%20%28single-precision%29))
  (bind _returnvalue (Math|Random|RandomFloat))
  (bind _returnvalue_2 (Math|Random|RandomFloat))
  (Utilities|FlowControl|Sequence
    (:then_0
      (Utilities|FlowControl|Delay (+ _returnvalue_2 1.0))
      (CallFunction|TailChange _returnvalue_2))
    (:then_1
      (Utilities|FlowControl|Delay (+ _returnvalue 1.0))
      (CallFunction|FinChange _returnvalue))))

(fn ConstructionScript)