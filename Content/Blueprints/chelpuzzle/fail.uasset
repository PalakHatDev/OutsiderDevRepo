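; Trigger box actor that handles failure in the chelpuzzle minigame when the puz_dude pawn overlaps it.
; On overlap it disables the pawn's input, shows the Fail widget and plays a timeline as a delay.
; When the timeline finishes, it clears all widgets, possesses the first-person character with input re-enabled, resets the pawn's Item to zero and hides the mouse cursor.
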(event OnComponentBeginOverlap(Box)
  (params (OverlappedComponent :type Primitive%20Component%20Object%20Reference) (OtherActor :type Actor%20Object%20Reference) (OtherComp :type Primitive%20Component%20Object%20Reference) (OtherBodyIndex :type Integer) (bFromSweep :type Boolean) (SweepResult :type Hit%20Result%20Structure%20%28by%20ref%29))
  (bind _returnvalue (Game|GetPlayerController 0))
  (bind _aspuz_dude (Utilities|Casting|CastTopuz_dude OtherActor))
  (Input|DisableInput _aspuz_dude (Game|GetPlayerController 0))
  (bind _returnvalue_2 (UserInterface|CreateWidget "/Game/Blueprints/Widgets/Fail.Fail_C"))
  (UserInterface|Viewport|AddtoViewport _returnvalue_2 0)
  (Timeline|Timeline PlayFromStart
    (:Finished
      (Viewport|RemoveAllWidgets)
      (bind _returnvalue_3 (Actor|GetActorOfClass "/Game/Blueprints/Player/BP_FirstPersonCharacter1.BP_FirstPersonCharacter1_C"))
      (Input|EnableInput _returnvalue_3 0)
      (Pawn|Possess _returnvalue _returnvalue_3)
      (bind _aspuz_dude_2 (Utilities|Casting|CastTopuz_dude OtherActor))
      (Variables|/Game/Blueprints/chelpuzzle/puz_dude.puz_dude_C|Setitem _aspuz_dude_2 0)
      (Variables|/Script/Engine.PlayerController|SetbShowMouseCursor _returnvalue false))))

(event EventBeginPlay)

(event Collision|EventActorBeginOverlap
  (params (OtherActor :type Actor%20Object%20Reference)))

(event EventTick
  (params (DeltaSeconds :type Float%20%28single-precision%29)))

(fn ConstructionScript)