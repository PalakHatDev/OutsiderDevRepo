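; Puz_spawn is a trigger actor that hands the player over from first-person play to a puzzle pawn.
; When BP_FirstPersonCharacter1 overlaps its Box, it disables that player's input, finds the Puz_dude and Cam actors by class, and has player controller 0 possess Puz_dude.
; It then switches the view target to Cam and shows the mouse cursor.
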(event OnComponentBeginOverlap(Box)
  (params (OverlappedComponent :type Primitive%20Component%20Object%20Reference) (OtherActor :type Actor%20Object%20Reference) (OtherComp :type Primitive%20Component%20Object%20Reference) (OtherBodyIndex :type Integer) (bFromSweep :type Boolean) (SweepResult :type Hit%20Result%20Structure%20%28by%20ref%29))
  (bind _asbp_first_person_character_1 (Utilities|Casting|CastToBP_FirstPersonCharacter1 OtherActor))
  (Input|DisableInput (Game|GetPlayerCharacter 0) (Game|GetPlayerController 0))
  (bind _asplayer_controller (Utilities|Casting|CastToPlayerController (Pawn|GetController _asbp_first_person_character_1)))
  (bind _returnvalue (Actor|GetActorOfClass "/Game/Blueprints/chelpuzzle/Cam.Cam_C"))
  (bind _returnvalue_2 (Actor|GetActorOfClass "/Game/Blueprints/chelpuzzle/puz_dude.puz_dude_C"))
  (Input|EnableInput _returnvalue_2 0)
  (Pawn|Possess (Game|GetPlayerController 0) _returnvalue_2)
  (Game|Player|SetViewTargetwithBlend _asplayer_controller _returnvalue 0.0 "VTBlend_Linear" 0.0 false)
  (Variables|/Script/Engine.PlayerController|SetbShowMouseCursor _asplayer_controller true))

(event EventBeginPlay)

(event Collision|EventActorBeginOverlap
  (params (OtherActor :type Actor%20Object%20Reference)))

(event EventTick
  (params (DeltaSeconds :type Float%20%28single-precision%29)))

(fn ConstructionScript)