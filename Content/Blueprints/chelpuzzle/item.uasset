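; Puzzle pickup item that the puz_dude character collects in a minigame.
; On sphere overlap it destroys itself, then increments the puz_dude's Item counter.
; When the count reaches three, it re-enables input on the first-person character and has the player controller possess it, ending the puzzle.
; Destruction happens before the cast, so any overlapping actor consumes the item.
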(event OnComponentBeginOverlap(Sphere1)
  (params (OverlappedComponent :type Primitive%20Component%20Object%20Reference) (OtherActor :type Actor%20Object%20Reference) (OtherComp :type Primitive%20Component%20Object%20Reference) (OtherBodyIndex :type Integer) (bFromSweep :type Boolean) (SweepResult :type Hit%20Result%20Structure%20%28by%20ref%29))
  (Actor|DestroyActor)
  (bind _aspuz_dude (Utilities|Casting|CastTopuz_dude OtherActor))
  (bind _output_get (Variables|/Game/Blueprints/chelpuzzle/puz_dude.puz_dude_C|Setitem _aspuz_dude (+ (Variables|/Game/Blueprints/chelpuzzle/puz_dude.puz_dude_C|Getitem _aspuz_dude) 1)))
  (if (== _output_get 3)
    (bind _returnvalue (Actor|GetActorOfClass "/Game/Blueprints/Player/BP_FirstPersonCharacter1.BP_FirstPersonCharacter1_C"))
    (Input|EnableInput _returnvalue 0)
    (Pawn|Possess (Game|GetPlayerController 0) _returnvalue)))

(event EventBeginPlay)

(event Collision|EventActorBeginOverlap
  (params (OtherActor :type Actor%20Object%20Reference)))

(event EventTick
  (params (DeltaSeconds :type Float%20%28single-precision%29)))

(fn ConstructionScript)