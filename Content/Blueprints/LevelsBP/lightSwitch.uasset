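; A light switch Blueprint that the player flips with the E key, animating its toggle.
; Both begin and end overlap enable input from player 0, so input is never disabled once gained.
; E flips the IsOn flag and plays or reverses a Timeline that drives the TogglePivot's relative pitch.
; The graph only animates the switch and does not control any light.
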(event Collision|EventActorBeginOverlap
  (params (OtherActor :type Actor%20Object%20Reference))
  (Input|EnableInput (Game|GetPlayerController 0)))

(event Collision|EventActorEndOverlap
  (params (OtherActor :type Actor%20Object%20Reference))
  (Input|EnableInput (Game|GetPlayerController 0)))

(event Input|KeyboardEvents|E
  (params (Key :type Key%20Structure))
  ;[1 1 1] Interaction with simple animation
  (:Pressed
    (if (Variables|Default|GetIsOn)
      (Variables|Default|SetIsOn false)
      (bind _newtrack_1 (Timeline|Timeline_0 Reverse)
        (:Update
          (Transformation|SetRelativeRotation (Variables|Default|GettogglePivot) (Math|Rotator|MakeRotator 0.0 _newtrack_1 0.0) false false)))
      (else
        (Variables|Default|SetIsOn true)
        (Timeline|Timeline_0 Play)))))

(fn ConstructionScript)