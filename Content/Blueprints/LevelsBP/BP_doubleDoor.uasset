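; Interactive double door that a player opens and closes with the E key while an actor overlaps it.
; Overlap events set an InputEnabled flag and toggle input through player controller 0.
; E flips IsOpen and plays an open or close timeline, rotating the two door pivots in opposite yaw directions.
; Input is disabled during the animation and restored on finish only if InputEnabled is still set.
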(event Collision|EventActorBeginOverlap
  (params (OtherActor :type Actor%20Object%20Reference))
  (Input|EnableInput (Game|GetPlayerController 0))
  (Variables|Default|SetinputEnabled true))

(event Collision|EventActorEndOverlap
  (params (OtherActor :type Actor%20Object%20Reference))
  (Input|DisableInput (Game|GetPlayerController 0) 0)
  (Variables|Default|SetinputEnabled false))

(event Input|KeyboardEvents|E
  (params (Key :type Key%20Structure))
  (bind _returnvalue (Game|GetPlayerController 0))
  (bind _rightdoorpivot (Variables|Default|GetrightDoorPivot))
  (bind _leftdoorpivot (Variables|Default|GetleftDoorPivot))
  ;[1 1 1] Interaction with simple animation
  (:Pressed
    (if (Variables|Default|GetisOpen)
      (Variables|Default|SetisOpen false)
      (bind _close (Timeline|Timeline_1 PlayFromStart)
        (:Update
          (Input|DisableInput _returnvalue)
          (Transformation|SetRelativeRotation _rightdoorpivot (Math|Rotator|MakeRotator 0.0 0.0 _close) false false)
          (Transformation|SetRelativeRotation _leftdoorpivot (Math|Rotator|MakeRotator 0.0 0.0 (* _close -1.0)) false false))
        (:Finished
          (if (Variables|Default|GetinputEnabled) :!label _label
            (Input|EnableInput _returnvalue))))
      (else
        (Variables|Default|SetisOpen true)
        (bind _open (Timeline|Timeline_0 PlayFromStart)
          (:Update
            (Input|DisableInput _returnvalue)
            (Transformation|SetRelativeRotation _rightdoorpivot (Math|Rotator|MakeRotator 0.0 0.0 _open) false false)
            (Transformation|SetRelativeRotation _leftdoorpivot (Math|Rotator|MakeRotator 0.0 0.0 (* _open -1.0)) false false))
          (:Finished
            (goto _label)))))))

(fn ConstructionScript)