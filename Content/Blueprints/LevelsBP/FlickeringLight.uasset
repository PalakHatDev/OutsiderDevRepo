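; A ceiling light actor that flickers endlessly with sparks and a looping sound.
; BeginPlay starts the sound at the actor and, after a random delay, enters Flicker, a self-repeating chain of random delays between TurnOff and TurnOn.
; Both toggle the RectLight's visibility and the mesh material together, and each switch-off in the cycle spawns a spark effect at the light.
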(event Custom|Flicker
  (CallFunction|TurnOff)
  (Niagara|SpawnSystematLocation "/Game/TMPDEVASSETS/Niagra/Spark.Spark" (Transformation|GetWorldLocation (Variables|Default|GetRectLight)))
  (Utilities|FlowControl|Delay (Math|Random|RandomFloatinRange 0.1 0.7))
  (CallFunction|Turnon)
  (Utilities|FlowControl|Delay (Math|Random|RandomFloatinRange 0.1 0.2))
  (CallFunction|TurnOff)
  (Niagara|SpawnSystematLocation "/Game/TMPDEVASSETS/Niagra/Spark.Spark" (Transformation|GetWorldLocation (Variables|Default|GetRectLight)))
  (Utilities|FlowControl|Delay (Math|Random|RandomFloatinRange 0.5 1.0))
  (CallFunction|Turnon)
  (Utilities|FlowControl|Delay (Math|Random|RandomFloatinRange 0.1 0.4))
  (CallFunction|Flicker))

(event Custom|TurnOff
  (Rendering|Material|SetMaterial (Variables|Default|GetStaticMesh) 0 0)
  (Rendering|SetVisibility (Variables|Default|GetRectLight) false false))

(event Custom|TurnOn
  (Rendering|Material|SetMaterial (Variables|Default|GetStaticMesh) 0 "/Game/GameAssets/Resources/HallwayProps/Materials/CeilingLight/MaT_ceilingLight20.MaT_ceilingLight20")
  (Rendering|SetVisibility (Variables|Default|GetRectLight) true false))

(event EventBeginPlay
  (Audio|PlaySoundatLocation "/Game/GameAssets/Resources/StarterContent/Audio/Light02_CueLooping.Light02_CueLooping" (Transformation|GetActorLocation) "0, 0, 0" 1.0 1.0 0.0 0 0 0 0)
  (Utilities|FlowControl|Delay (Math|Random|RandomFloatinRange 0.1 0.5))
  (CallFunction|TurnOff)
  (Niagara|SpawnSystematLocation "/Game/TMPDEVASSETS/Niagra/Spark.Spark" (Transformation|GetWorldLocation (Variables|Default|GetRectLight)))
  (Utilities|FlowControl|Delay (Math|Random|RandomFloatinRange 0.1 0.7))
  (CallFunction|Turnon)
  (Utilities|FlowControl|Delay (Math|Random|RandomFloatinRange 0.1 0.2))
  (CallFunction|TurnOff)
  (Niagara|SpawnSystematLocation "/Game/TMPDEVASSETS/Niagra/Spark.Spark" (Transformation|GetWorldLocation (Variables|Default|GetRectLight)))
  (Utilities|FlowControl|Delay (Math|Random|RandomFloatinRange 0.5 1.0))
  (CallFunction|Turnon)
  (Utilities|FlowControl|Delay (Math|Random|RandomFloatinRange 0.1 0.4))
  (CallFunction|Flicker))

(fn ConstructionScript)