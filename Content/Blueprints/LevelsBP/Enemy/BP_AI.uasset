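; BP_AI is an enemy pawn that roams the navmesh, chases pawns it sees, and damages any actor overlapping its capsule.
; Roaming repeatedly walks to random reachable points, restarting on each successful move.
; PawnSensing switches it to a faster chase, with each state setting its own materials and animation and posting an audio event.
; A retriggerable delay returns it to roaming shortly after sightings stop.
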(event OnSeePawn(PawnSensing)
  (params (Pawn :type Pawn%20Object%20Reference))
  (bind _mesh (Variables|Character|GetMesh))
  (CallFunction|PostEvent)
  (Rendering|Material|SetMaterial _mesh 0 "/Game/TMPDEVASSETS/StarterContent/Materials/M_Tech_HexTileRed_Chasing.M_Tech_HexTileRed_Chasing")
  (Rendering|Material|SetMaterial _mesh 1 "/Game/TMPDEVASSETS/StarterContent/Materials/M_Tech_HexTileRed_Chasing.M_Tech_HexTileRed_Chasing")
  (Components|Animation|PlayAnimation (Variables|Character|GetMesh) "/Game/GameAssets/Resources/Characters/Mannequins/Animations/Manny/MM_Run_Fwd.MM_Run_Fwd" false)
  (Variables|/Script/Engine.CharacterMovementComponent|SetMaxWalkSpeed (Variables|Character|GetCharacterMovement) 7e+02)
  (Utilities|FlowControl|Sequence
    (:then_0
      (AI|AIMoveTo self "0, 0, 0" Pawn 5.0 false))
    (:then_1
      (Utilities|FlowControl|RetriggerableDelay 2.5)
      (CallFunction|StartRoam))))

(event Custom|StartRoam
  (bind _mesh (Variables|Character|GetMesh))
  (CallFunction|PostEvent)
  (Rendering|Material|SetMaterial _mesh 0 "/Game/TMPDEVASSETS/StarterContent/Materials/M_Tech_HexTileRed_Roaming.M_Tech_HexTileRed_Roaming")
  (Rendering|Material|SetMaterial _mesh 1 "/Game/TMPDEVASSETS/StarterContent/Materials/M_Tech_HexTileRed_Roaming.M_Tech_HexTileRed_Roaming")
  (Components|Animation|PlayAnimation (Variables|Character|GetMesh) "/Game/GameAssets/Resources/Characters/Mannequins/Animations/Manny/MM_Walk_Fwd.MM_Walk_Fwd" false)
  (Variables|/Script/Engine.CharacterMovementComponent|SetMaxWalkSpeed (Variables|Character|GetCharacterMovement) 3e+02)
  (AI|AIMoveTo self (.RandomLocation (AI|Navigation|GetRandomReachablePointinRadius (Transformation|GetActorLocation) 2.5e+03 0 "/Script/AIModule.NavFilter_AIControllerDefault")) 0 5.0 false
    (:OnSuccess
      (CallFunction|StartRoam))))

(event Custom|OnComponentBeginOverlap_Event
  (params (OverlappedComponent :type Primitive%20Component%20Object%20Reference) (OtherActor :type Actor%20Object%20Reference) (OtherComp :type Primitive%20Component%20Object%20Reference) (OtherBodyIndex :type Integer) (bFromSweep :type Boolean) (SweepResult :type Hit%20Result%20Structure%20%28by%20ref%29))
  (Game|Damage|ApplyDamage OtherActor 1e+02 0 self))

(event EventBeginPlay
  (CallFunction|StartRoam)
  (Collision|AssignOnComponentBeginOverlap (Variables|Default|GetCapsule) (delegate Custom|OnComponentBeginOverlap_Event)))

(fn ConstructionScript)